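; Enemy character Blueprint that handles the enemy's animation speed, ragdoll and explosive death.
; Tick scales mesh play rate by max movement speed, and BeginPlay attaches a collision component to the capsule.
; Ragdoll blends physics below a bone via PhysicalAnimation, exploding cosmetically if health is depleted, while Die halts movement and triggers a damaging explosion.
; Both paths share a delayed sound-and-destroy tail with a rare heal drop requiring the Killed flag.
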(event OnComponentBeginOverlap(Sphere)
  (params (OverlappedComponent :type Primitive%20Component%20Object%20Reference) (OtherActor :type Actor%20Object%20Reference) (OtherComp :type Primitive%20Component%20Object%20Reference) (OtherBodyIndex :type Integer) (bFromSweep :type Boolean) (SweepResult :type Hit%20Result%20Structure%20%28by%20ref%29)))

(event EventBeginPlay
  (Transformation|SetWorldLocation (Variables|Default|GetCollisionComp) (Transformation|GetWorldLocation (Variables|Default|GetCapsuleComponent)) false true)
  (Transformation|AttachComponentToComponent (Variables|Default|GetCollisionComp) (Variables|Default|GetCapsuleComponent) "None" "SnapToTarget" "KeepRelative" "KeepRelative" true))

(event Collision|EventActorBeginOverlap
  (params (OtherActor :type Actor%20Object%20Reference)))

(event EventTick
  (params (DeltaSeconds :type Float%20%28single-precision%29))
  (Components|Timeline|SetPlayRate (Variables|Character|GetMesh) (/ (Class|MovementComponent|GetMaxSpeed (Variables|Character|GetCharacterMovement)) 9e+02)))

(event EventDie
  (bind _returnvalue (Transformation|GetActorLocation))
  (bind _returnvalue_2 (Transformation|GetActorLocation))
  (Pawn|Components|CharacterMovement|DisableMovement (Variables|Character|GetCharacterMovement))
  (Utilities|FlowControl|Delay 1.0)
  (bind _returnvalue_3 (AddComponent|AddGenericExplosive))
  (Default|SetupExplosion _returnvalue_3 3e+02 75.0)
  (Default|Explosion _returnvalue_3 _returnvalue)
  (Effects|SpawnEmitteratLocation "/Game/StarterContent/Particles/P_Explosion_2.P_Explosion_2" _returnvalue)
  (Audio|SpawnSoundatLocation "/Game/EnemyStuff/Explosion1.Explosion1" _returnvalue_2)
  (if (> (Math|Random|RandomIntegerinRange 0 10) 9)
    (if (Variables|Default|GetKilled)
      (Game|SpawnActorfromClass "/Game/EnemyStuff/HealDrop.HealDrop_C" (Math|Conversions|ToTransform(Vector) _returnvalue_2) "Undefined" 0 0)
      (Actor|DestroyActor :!label _label))
    (else
      (goto _label))))

(event EventRagdoll
  (bind _returnvalue (Transformation|GetActorLocation))
  (bind _physicalanimation (Variables|Default|GetPhysicalAnimation))
  (bind _mesh (Variables|Character|GetMesh))
  (bind _bonename (Variables|Default|Getbonename))
  (Variables|Default|SetKilled true)
  (Class|PhysicalAnimationComponent|SetSkeletalMeshComponent _physicalanimation _mesh)
  (Class|PhysicalAnimationComponent|ApplyPhysicalAnimationProfileBelow _physicalanimation _bonename "None" true false)
  (Class|SkeletalMeshComponent|SetAllBodiesBelowSimulatePhysics _mesh _bonename true true)
  (Utilities|FlowControl|Delay 1.0)
  (if (<= (Variables|Default|Gethealth) 0)
    (Effects|SpawnEmitteratLocation "/Game/StarterContent/Particles/P_Explosion_2.P_Explosion_2" _returnvalue)
    (Audio|SpawnSoundatLocation "/Game/EnemyStuff/Explosion1.Explosion1" _returnvalue)
    (if (> (Math|Random|RandomIntegerinRange 0 10) 9)
      (if (Variables|Default|GetKilled)
        (Game|SpawnActorfromClass "/Game/EnemyStuff/HealDrop.HealDrop_C" (Math|Conversions|ToTransform(Vector) _returnvalue) "Undefined" 0 0)
        (Actor|DestroyActor :!label _label))
      (else
        (goto _label)))))

(fn ConstructionScript)

(fn NewFunction0)