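; Walker enemy character that can ragdoll, drop healing and explode on death.
; Tick scales mesh play rate to max movement speed, and BeginPlay snaps CollisionComp onto the capsule.
; Ragdoll simulates physics below a bone with physical animation, then, if health is depleted, may spawn HealDrop before destroying the actor with effects.
; Die halts movement, waits, triggers a damaging GenericExplosive, and shares that effects-and-destroy tail without the drop.
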(event OnComponentBeginOverlap(Sphere)
  (params (OverlappedComponent :type Primitive%20Component%20Object%20Reference) (OtherActor :type Actor%20Object%20Reference) (OtherComp :type Primitive%20Component%20Object%20Reference) (OtherBodyIndex :type Integer) (bFromSweep :type Boolean) (SweepResult :type Hit%20Result%20Structure%20%28by%20ref%29)))

(event EventBeginPlay
  (Transformation|SetWorldLocation (Variables|Default|GetCollisionComp) (Transformation|GetWorldLocation (Variables|Default|GetCapsuleComponent)) false true)
  (Transformation|AttachComponentToComponent (Variables|Default|GetCollisionComp) (Variables|Default|GetCapsuleComponent) "None" "SnapToTarget" "KeepRelative" "KeepRelative" true))

(event Collision|EventActorBeginOverlap
  (params (OtherActor :type Actor%20Object%20Reference)))

(event EventTick
  (params (DeltaSeconds :type Float%20%28single-precision%29))
  (Components|Timeline|SetPlayRate (Variables|Character|GetMesh) (/ (Class|MovementComponent|GetMaxSpeed (Variables|Character|GetCharacterMovement)) 9e+02)))

(event EventDie
  (Pawn|Components|CharacterMovement|DisableMovement (Variables|Character|GetCharacterMovement))
  (Utilities|FlowControl|Delay 1.0)
  (bind _returnvalue (AddComponent|AddGenericExplosive))
  (Default|SetupExplosion _returnvalue 3e+02 75.0)
  (Default|Explosion _returnvalue (Transformation|GetActorLocation))
  (Effects|SpawnEmitteratLocation "/Game/StarterContent/Particles/P_Explosion_2.P_Explosion_2" (Transformation|GetWorldLocation (Variables|Character|GetMesh)))
  (Audio|SpawnSoundatLocation "/Game/EnemyStuff/Walker/Explosion1.Explosion1" "0, 0, 0")
  (Actor|DestroyActor))

(event EventRagdoll
  (bind _physicalanimation (Variables|Default|GetPhysicalAnimation))
  (bind _mesh (Variables|Character|GetMesh))
  (bind _bonename (Variables|Default|Getbonename))
  (Variables|Default|SetKilled true)
  (Class|PhysicalAnimationComponent|SetSkeletalMeshComponent _physicalanimation _mesh)
  (Class|PhysicalAnimationComponent|ApplyPhysicalAnimationProfileBelow _physicalanimation _bonename "None" true false)
  (Class|SkeletalMeshComponent|SetAllBodiesBelowSimulatePhysics _mesh _bonename true true)
  (Utilities|FlowControl|Delay 1.0)
  (if (<= (Variables|Default|Gethealth) 0)
    (if (> (Math|Random|RandomIntegerinRange 0 10) 7)
      (if (Variables|Default|GetKilled)
        (Game|SpawnActorfromClass "/Game/EnemyStuff/Walker/HealDrop.HealDrop_C" (Math|Conversions|ToTransform(Vector) (Transformation|GetActorLocation)) "Undefined" 0 0)
        (Effects|SpawnEmitteratLocation "/Game/StarterContent/Particles/P_Explosion_2.P_Explosion_2" (Transformation|GetWorldLocation (Variables|Character|GetMesh)) :!label _label)
        (Audio|SpawnSoundatLocation "/Game/EnemyStuff/Walker/Explosion1.Explosion1" "0, 0, 0")
        (Actor|DestroyActor))
      (else
        (goto _label)))))

(fn ConstructionScript)

(fn NewFunction0)