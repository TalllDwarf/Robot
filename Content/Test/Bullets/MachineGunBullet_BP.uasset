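; MachineGunBullet_BP is a machine gun projectile that damages enemy characters on contact.
; When its box collision begins an overlap, an EnemyCharacterBP takes the truncated Damage value and a small push along the bullet's forward vector through its movement component.
; Any overlap, enemy or not, spawns the BulletLine particle effect at the bullet's location and destroys the bullet.
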(event OnComponentBeginOverlap(boxCollision)
  (params (OverlappedComponent :type Primitive%20Component%20Object%20Reference) (OtherActor :type Actor%20Object%20Reference) (OtherComp :type Primitive%20Component%20Object%20Reference) (OtherBodyIndex :type Integer) (bFromSweep :type Boolean) (SweepResult :type Hit%20Result%20Structure%20%28by%20ref%29))
  (bind _asenemy_character_bp (Utilities|Casting|CastToEnemyCharacterBP OtherActor)
    (:then
      (Class|EnemyCharacter|TakeDamage _asenemy_character_bp (Math|Float|Truncate (Variables|Default|Getdamage)))
      (Physics|AddImpulse (Variables|/Script/Engine.Character|GetCharacterMovement _asenemy_character_bp) (* (Transformation|GetActorForwardVector) 100) false))
    (:CastFailed
      _))
  (Effects|SpawnEmitteratLocation "/Game/Test/BulletLine.BulletLine" (Transformation|GetActorLocation))
  (Actor|DestroyActor))

(fn ConstructionScript)