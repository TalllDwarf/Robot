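; JunkGun_BP is a shotgun-style gun Blueprint that fires several JunkBullet actors per shot with random spread.
; Shoot is gated by a cooldown and an IsActive check, adds heat, then spawns muzzle smoke and bullets at the PointLight.
; Each bullet's rotation comes from randomly jittering the light's forward vector.
; Tick counts down the cooldown and switches off the muzzle-flash light halfway through the shot delay.
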(event EventTick
  (params (DeltaSeconds :type Float%20%28single-precision%29))
  (|CallParentFunction DeltaSeconds)
  ;[1 1 1] Shoot delay
  (if (> (Variables|Default|GetCurrentShotDelay) 0.0)
    (Variables|Default|SetCurrentShotDelay (- (Variables|Default|GetCurrentShotDelay) DeltaSeconds)))
  ;[1 1 1] Turn light off
  (if (< (Variables|Default|GetLightOnLeft) 0.0)
    ;[1 1 1] Turn light off
    (Rendering|Components|Light|SetIntensity (Variables|Default|GetPointLight) 0.0)
    (else
      (Variables|Default|SetLightOnLeft (- (Variables|Default|GetLightOnLeft) DeltaSeconds)))))

(event EventShoot
  (bind _pointlight (Variables|Default|GetPointLight))
  (bind _pointlight_2 (Variables|Default|GetPointLight))
  (bind _returnvalue (Transformation|GetWorldTransform _pointlight))
  (bind _returnvalue_2 (Math|Vector|GetForwardVector (.rotation _returnvalue)))
  ;[1 1 1] Can we shoot
  (if (<= (Variables|Default|GetCurrentShotDelay) 0.0)
    (bind _returnvalue_3 (Class|RobotGun|IsActive))
    (if _returnvalue_3
      (Class|RobotGun|AddHeat (* (Variables|Default|GetHeatMult) 9.0))
      (Variables|Default|SetCurrentShotDelay (Variables|Default|GetShotDelay))
      ;[1 1 1] Flash light
      (Variables|Default|SetLightOnLeft (/ (Variables|Default|GetShotDelay) 2.0))
      (Rendering|Components|Light|SetIntensity _pointlight_2 3e+03)
      ;[1 1 1] spawn muzzle smoke
      (Effects|SpawnEmitteratLocation "/Game/StarterContent/Particles/muzzle.muzzle" (.location (Transformation|GetWorldTransform _pointlight_2)))
      ;[1 1 1] spawn bullets with a slight spread
      (for _index (range 0 (Variables|Default|GetbulletsPerShot))
        (Game|SpawnActorfromClass "/Game/Test/Bullets/JunkBullet.JunkBullet_C" (Math|Transform|MakeTransform (.location _returnvalue) (Math|Rotator|FindLookatRotation (.location _returnvalue) (+ (.location _returnvalue) (Math|Vector|MakeVector (+ (.x _returnvalue_2) (Math|Random|RandomFloatinRange -0.06 0.06)) (+ (.y _returnvalue_2) (Math|Random|RandomFloatinRange -0.06 0.06)) (+ (.z _returnvalue_2) (Math|Random|RandomFloatinRange -0.06 0.06))))) (.scale _returnvalue)) "Undefined" 0 0)))))

(fn ConstructionScript
  (|CallParentFunction))