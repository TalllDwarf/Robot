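; Test Blueprint for a tracked leg assembly that animates six wheels, three on the left and three on the right.
; Each tick, while ShouldWheelsSpin is true, it pitches every wheel at a constant rate scaled by delta time, independent of speed.
; An unconnected branch that would play or stop audio based on velocity never runs, and the construction script is empty.
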(event EventTick
  (params (DeltaSeconds :type Float%20%28single-precision%29))
  ;[1 1 1] Turn wheels
  (if (Class|RobotLegPart|ShouldWheelsSpin)
    (for _array_element (Utilities|Array|MakeArray (Variables|Default|GetLeftWheelFront) (Variables|Default|GetLeftWheelMiddle) (Variables|Default|GetLeftWheelBack) (Variables|Default|GetRightWheelFront) (Variables|Default|GetRightWheelMiddle) (Variables|Default|GetRightWheelBack))
      (Transformation|AddLocalRotation _array_element (Math|Rotator|MakeRotator 0.0 (* DeltaSeconds 1.5e+02) 0.0) false false))))

(fn ConstructionScript)